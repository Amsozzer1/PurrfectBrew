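; Modular customizable character that cycles skeletal meshes for shoes, facial hair, accessories, bottoms, tops, hats, hair and faces.
; Next/Prev functions step each slot's wrapping index through its options array and swap that mesh component.
; Save and Load functions store indices in BP_CharacterSave; loading omits TopIndex and does not reapply meshes.
; Setup that fills the arrays, creates WBP_CharacterCustomizer and loads the save is disconnected, so BeginPlay does nothing.
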(event EventBeginPlay)

(event Collision|EventActorBeginOverlap
  (params (OtherActor :type Actor%20Object%20Reference)))

(event EventTick
  (params (DeltaSeconds :type Float%20%28single-precision%29)))

(fn ConstructionScript)

(fn NextShoe
  (Variables|Default|SetShoeIndex (Math|Integer|%(Integer) (+ (Variables|Default|GetShoeIndex) 1) (Utilities|Array|Length (Variables|Default|GetShoeOptions))))
  (Components|SkeletalMesh|SetSkeletalMeshAsset (Variables|Default|GetShoeMesh) (Utilities|Array|Get(acopy) (Variables|Default|GetShoeOptions) (Variables|Default|GetShoeIndex))))

(fn PrevShoe
  (if (< (- (Variables|Default|GetShoeIndex) 1) 0)
    (Variables|Default|SetShoeIndex (- (Utilities|Array|Length (Variables|Default|GetShoeOptions)) 1))
    (Components|SkeletalMesh|SetSkeletalMeshAsset (Variables|Default|GetShoeMesh) (Utilities|Array|Get(acopy) (Variables|Default|GetShoeOptions) (Variables|Default|GetShoeIndex)))
    (else
      (Variables|Default|SetShoeIndex (Math|Integer|%(Integer) (- (Variables|Default|GetShoeIndex) 1) (Utilities|Array|Length (Variables|Default|GetShoeOptions))))
      (Components|SkeletalMesh|SetSkeletalMeshAsset (Variables|Default|GetShoeMesh) (Utilities|Array|Get(acopy) (Variables|Default|GetShoeOptions) (Variables|Default|GetShoeIndex))))))

(fn NextFacialHair
  (Variables|Default|SetFacialHairIndex (Math|Integer|%(Integer) (+ (Variables|Default|GetFacialHairIndex) 1) (Utilities|Array|Length (Variables|Default|GetFacialHairOptions))))
  (Components|SkeletalMesh|SetSkeletalMeshAsset (Variables|Default|GetFacialHairMesh) (Utilities|Array|Get(acopy) (Variables|Default|GetFacialHairOptions) (Variables|Default|GetFacialHairIndex))))

(fn PrevFacialHair
  (if (< (- (Variables|Default|GetFacialHairIndex) 1) 0)
    (Variables|Default|SetFacialHairIndex (- (Utilities|Array|Length (Variables|Default|GetFacialHairOptions)) 1))
    (Components|SkeletalMesh|SetSkeletalMeshAsset (Variables|Default|GetFacialHairMesh) (Utilities|Array|Get(acopy) (Variables|Default|GetFacialHairOptions) (Variables|Default|GetFacialHairIndex)))
    (else
      (Variables|Default|SetFacialHairIndex (Math|Integer|%(Integer) (- (Variables|Default|GetFacialHairIndex) 1) (Utilities|Array|Length (Variables|Default|GetFacialHairOptions))))
      (Components|SkeletalMesh|SetSkeletalMeshAsset (Variables|Default|GetFacialHairMesh) (Utilities|Array|Get(acopy) (Variables|Default|GetFacialHairOptions) (Variables|Default|GetFacialHairIndex))))))

(fn NextAccessory
  (Variables|Default|SetAccessoryIndex (Math|Integer|%(Integer) (+ (Variables|Default|GetAccessoryIndex) 1) (Utilities|Array|Length (Variables|Default|GetAccessoryOptions))))
  (Components|SkeletalMesh|SetSkeletalMeshAsset (Variables|Default|GetGlassesMesh) (Utilities|Array|Get(acopy) (Variables|Default|GetAccessoryOptions) (Variables|Default|GetAccessoryIndex))))

(fn PrevAccessory
  (if (< (- (Variables|Default|GetAccessoryIndex) 1) 0)
    (Variables|Default|SetAccessoryIndex (- (Utilities|Array|Length (Variables|Default|GetAccessoryOptions)) 1))
    (Components|SkeletalMesh|SetSkeletalMeshAsset (Variables|Default|GetGlassesMesh) (Utilities|Array|Get(acopy) (Variables|Default|GetAccessoryOptions) (Variables|Default|GetAccessoryIndex)))
    (else
      (Variables|Default|SetAccessoryIndex (Math|Integer|%(Integer) (- (Variables|Default|GetAccessoryIndex) 1) (Utilities|Array|Length (Variables|Default|GetAccessoryOptions))))
      (Components|SkeletalMesh|SetSkeletalMeshAsset (Variables|Default|GetGlassesMesh) (Utilities|Array|Get(acopy) (Variables|Default|GetAccessoryOptions) (Variables|Default|GetAccessoryIndex))))))

(fn NextBottom
  (Variables|Default|SetBottomIndex (Math|Integer|%(Integer) (+ (Variables|Default|GetBottomIndex) 1) (Utilities|Array|Length (Variables|Default|GetBottomOptions))))
  (Components|SkeletalMesh|SetSkeletalMeshAsset (Variables|Default|GetBottommesh) (Utilities|Array|Get(acopy) (Variables|Default|GetBottomOptions) (Variables|Default|GetBottomIndex))))

(fn PrevBottom
  (if (< (- (Variables|Default|GetBottomIndex) 1) 0)
    (Variables|Default|SetBottomIndex (- (Utilities|Array|Length (Variables|Default|GetBottomOptions)) 1))
    (Components|SkeletalMesh|SetSkeletalMeshAsset (Variables|Default|GetBottommesh) (Utilities|Array|Get(acopy) (Variables|Default|GetBottomOptions) (Variables|Default|GetBottomIndex)))
    (else
      (Variables|Default|SetBottomIndex (Math|Integer|%(Integer) (- (Variables|Default|GetBottomIndex) 1) (Utilities|Array|Length (Variables|Default|GetBottomOptions))))
      (Components|SkeletalMesh|SetSkeletalMeshAsset (Variables|Default|GetBottommesh) (Utilities|Array|Get(acopy) (Variables|Default|GetBottomOptions) (Variables|Default|GetBottomIndex))))))

(fn NextTop
  (Variables|Default|SetTopIndex (Math|Integer|%(Integer) (+ (Variables|Default|GetTopIndex) 1) (Utilities|Array|Length (Variables|Default|GetTopOptions))))
  (Components|SkeletalMesh|SetSkeletalMeshAsset (Variables|Default|GetTopMesh) (Utilities|Array|Get(acopy) (Variables|Default|GetTopOptions) (Variables|Default|GetTopIndex))))

(fn PrevTop
  (if (< (- (Variables|Default|GetTopIndex) 1) 0)
    (Variables|Default|SetTopIndex (- (Utilities|Array|Length (Variables|Default|GetTopOptions)) 1))
    (Components|SkeletalMesh|SetSkeletalMeshAsset (Variables|Default|GetTopMesh) (Utilities|Array|Get(acopy) (Variables|Default|GetTopOptions) (Variables|Default|GetTopIndex)))
    (else
      (Variables|Default|SetTopIndex (Math|Integer|%(Integer) (- (Variables|Default|GetTopIndex) 1) (Utilities|Array|Length (Variables|Default|GetBottomOptions))))
      (Components|SkeletalMesh|SetSkeletalMeshAsset (Variables|Default|GetTopMesh) (Utilities|Array|Get(acopy) (Variables|Default|GetTopOptions) (Variables|Default|GetTopIndex))))))

(fn NextHat
  (Variables|Default|SetHatIndex (Math|Integer|%(Integer) (+ (Variables|Default|GetHatIndex) 1) (Utilities|Array|Length (Variables|Default|GetHatOptions))))
  (Components|SkeletalMesh|SetSkeletalMeshAsset (Variables|Default|GetHatMesh) (Utilities|Array|Get(acopy) (Variables|Default|GetHatOptions) (Variables|Default|GetHatIndex))))

(fn PrevHat
  (if (< (- (Variables|Default|GetHatIndex) 1) 0)
    (Variables|Default|SetHatIndex (- (Utilities|Array|Length (Variables|Default|GetHatOptions)) 1))
    (Components|SkeletalMesh|SetSkeletalMeshAsset (Variables|Default|GetHatMesh) (Utilities|Array|Get(acopy) (Variables|Default|GetHatOptions) (Variables|Default|GetHatIndex)))
    (else
      (Variables|Default|SetHatIndex (Math|Integer|%(Integer) (- (Variables|Default|GetHatIndex) 1) (Utilities|Array|Length (Variables|Default|GetHatOptions))))
      (Components|SkeletalMesh|SetSkeletalMeshAsset (Variables|Default|GetHatMesh) (Utilities|Array|Get(acopy) (Variables|Default|GetHatOptions) (Variables|Default|GetHatIndex))))))

(fn NextHair
  (Variables|Default|SetHairIndex (Math|Integer|%(Integer) (+ (Variables|Default|GetHairIndex) 1) (Utilities|Array|Length (Variables|Default|GetHairOptions))))
  (Components|SkeletalMesh|SetSkeletalMeshAsset (Variables|Default|GetHairMesh) (Utilities|Array|Get(acopy) (Variables|Default|GetHairOptions) (Variables|Default|GetHairIndex))))

(fn PrevHair
  (if (< (- (Variables|Default|GetHairIndex) 1) 0)
    (Variables|Default|SetHairIndex (- (Utilities|Array|Length (Variables|Default|GetHairOptions)) 1))
    (Components|SkeletalMesh|SetSkeletalMeshAsset (Variables|Default|GetHairMesh) (Utilities|Array|Get(acopy) (Variables|Default|GetHairOptions) (Variables|Default|GetHairIndex)))
    (else
      (Variables|Default|SetHairIndex (Math|Integer|%(Integer) (- (Variables|Default|GetHairIndex) 1) (Utilities|Array|Length (Variables|Default|GetHairOptions))))
      (Components|SkeletalMesh|SetSkeletalMeshAsset (Variables|Default|GetHairMesh) (Utilities|Array|Get(acopy) (Variables|Default|GetHairOptions) (Variables|Default|GetHairIndex))))))

(fn NextFace
  (Variables|Default|SetFaceIndex (Math|Integer|%(Integer) (+ (Variables|Default|GetFaceIndex) 1) (Utilities|Array|Length (Variables|Default|GetFaceOptions))))
  (Components|SkeletalMesh|SetSkeletalMeshAsset (Variables|Default|GetFaceMesh) (Utilities|Array|Get(acopy) (Variables|Default|GetFaceOptions) (Variables|Default|GetFaceIndex))))

(fn PrevFace
  (if (< (- (Variables|Default|GetFaceIndex) 1) 0)
    (Variables|Default|SetFaceIndex (- (Utilities|Array|Length (Variables|Default|GetFaceOptions)) 1))
    (Components|SkeletalMesh|SetSkeletalMeshAsset (Variables|Default|GetFaceMesh) (Utilities|Array|Get(acopy) (Variables|Default|GetFaceOptions) (Variables|Default|GetFaceIndex)))
    (else
      (Variables|Default|SetFaceIndex (Math|Integer|%(Integer) (- (Variables|Default|GetFaceIndex) 1) (Utilities|Array|Length (Variables|Default|GetFaceOptions))))
      (Components|SkeletalMesh|SetSkeletalMeshAsset (Variables|Default|GetFaceMesh) (Utilities|Array|Get(acopy) (Variables|Default|GetFaceOptions) (Variables|Default|GetFaceIndex))))))

(fn LoadCustomization
  (bind _returnvalue (SaveGame|DoesSaveGameExist "CharacterCustomization"))
  (if _returnvalue
    (bind _returnvalue_2 (SaveGame|LoadGamefromSlot "CharacterCustomization"))
    (bind _asbp_character_save (Utilities|Casting|CastToBP_CharacterSave _returnvalue_2))
    (Variables|Default|SetShoeIndex (Variables|/Game/UI/BP_CharacterSave.BP_CharacterSave_C|GetShoeIndex _asbp_character_save))
    (Variables|Default|SetFacialHairIndex (Variables|/Game/UI/BP_CharacterSave.BP_CharacterSave_C|GetFacialHairIndex _asbp_character_save))
    (Variables|Default|SetAccessoryIndex (Variables|/Game/UI/BP_CharacterSave.BP_CharacterSave_C|GetAccessoryIndex _asbp_character_save))
    (Variables|Default|SetBottomIndex (Variables|/Game/UI/BP_CharacterSave.BP_CharacterSave_C|GetBottomIndex _asbp_character_save))
    (Variables|Default|SetHairIndex (Variables|/Game/UI/BP_CharacterSave.BP_CharacterSave_C|GetHairIndex _asbp_character_save))
    (Variables|Default|SetHatIndex (Variables|/Game/UI/BP_CharacterSave.BP_CharacterSave_C|GetHatIndex _asbp_character_save))
    (Variables|Default|SetFaceIndex (Variables|/Game/UI/BP_CharacterSave.BP_CharacterSave_C|GetFaceIndex _asbp_character_save))))

(fn SaveCustomization
  (bind _returnvalue (SaveGame|CreateSaveGameObject "/Game/UI/BP_CharacterSave.BP_CharacterSave_C"))
  (Variables|/Game/UI/BP_CharacterSave.BP_CharacterSave_C|SetShoeIndex _returnvalue (Variables|Default|GetShoeIndex))
  (Variables|/Game/UI/BP_CharacterSave.BP_CharacterSave_C|SetFacialHairIndex _returnvalue (Variables|Default|GetFacialHairIndex))
  (Variables|/Game/UI/BP_CharacterSave.BP_CharacterSave_C|SetAccessoryIndex _returnvalue (Variables|Default|GetAccessoryIndex))
  (Variables|/Game/UI/BP_CharacterSave.BP_CharacterSave_C|SetBottomIndex _returnvalue (Variables|Default|GetBottomIndex))
  (Variables|/Game/UI/BP_CharacterSave.BP_CharacterSave_C|SetTopIndex _returnvalue (Variables|Default|GetTopIndex))
  (Variables|/Game/UI/BP_CharacterSave.BP_CharacterSave_C|SetHairIndex _returnvalue (Variables|Default|GetHairIndex))
  (Variables|/Game/UI/BP_CharacterSave.BP_CharacterSave_C|SetHatIndex _returnvalue (Variables|Default|GetHatIndex))
  (Variables|/Game/UI/BP_CharacterSave.BP_CharacterSave_C|SetFaceIndex _returnvalue (Variables|Default|GetFaceIndex))
  (SaveGame|SaveGametoSlot _returnvalue "CharacterCustomization"))