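; Cat café coffee machine that brews the player's chosen beverage and grades it against the linked cashier's NPC order.
; Player overlap opens the BP_CoffeeMenu widget with UI-only input.
; Tick polls MenuButtonClicked, spawns a beverage with the menu's choices, waits, then moves it to a fixed position.
; Nested branches match hardcoded order strings, set cashier result flags and destroy the drink; sugar without cream has no branch.
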(event OnClicked(Machine)
  (params (TouchedComponent :type Primitive%20Component%20Object%20Reference) (ButtonPressed :type Key%20Structure :default "None")))

(event OnComponentBeginOverlap(Machine)
  (params (OverlappedComponent :type Primitive%20Component%20Object%20Reference) (OtherActor :type Actor%20Object%20Reference) (OtherComp :type Primitive%20Component%20Object%20Reference) (OtherBodyIndex :type Integer) (bFromSweep :type Boolean) (SweepResult :type Hit%20Result%20Structure%20%28by%20ref%29))
  (bind _returnvalue (Game|GetPlayerController 0))
  (Utilities|Casting|CastToBP_ThirdPersonCharacter (stale OnComponentBeginOverlap(Box) OtherActor))
  (bind _returnvalue_2 (UserInterface|CreateWidget "/Game/Catcafe/meshes/BP_CoffeeMenu.BP_CoffeeMenu_C"))
  (Variables|/Game/Catcafe/meshes/BP_CoffeeMenu.BP_CoffeeMenu_C|SetSourceMachine _returnvalue_2 self)
  (UserInterface|Viewport|AddtoViewport _returnvalue_2 0)
  (Input|SetInputModeUIOnly _returnvalue 0 "DoNotLock" false)
  (Variables|/Script/Engine.PlayerController|SetbShowMouseCursor _returnvalue false))

(event OnComponentBeginOverlap(Box)
  (params (OverlappedComponent :type Primitive%20Component%20Object%20Reference) (OtherActor :type Actor%20Object%20Reference) (OtherComp :type Primitive%20Component%20Object%20Reference) (OtherBodyIndex :type Integer) (bFromSweep :type Boolean) (SweepResult :type Hit%20Result%20Structure%20%28by%20ref%29))
  (bind _returnvalue (Game|GetPlayerController 0))
  (Utilities|Casting|CastToBP_ThirdPersonCharacter OtherActor)
  (bind _returnvalue_2 (UserInterface|CreateWidget "/Game/Catcafe/meshes/BP_CoffeeMenu.BP_CoffeeMenu_C"))
  (Variables|/Game/Catcafe/meshes/BP_CoffeeMenu.BP_CoffeeMenu_C|SetSourceMachine _returnvalue_2 self)
  (UserInterface|Viewport|AddtoViewport _returnvalue_2 0)
  (Input|SetInputModeUIOnly _returnvalue 0 "DoNotLock" false)
  (Variables|/Script/Engine.PlayerController|SetbShowMouseCursor _returnvalue false))

(event EventBeginPlay)

(event Collision|EventActorBeginOverlap
  (params (OtherActor :type Actor%20Object%20Reference)))

(event EventTick
  (params (DeltaSeconds :type Float%20%28single-precision%29))
  (bind _linkedcashier (Variables|Default|GetLinkedCashier))
  (bind _linkedcashier_2 (Variables|Default|GetLinkedCashier))
  (bind _linkedcashier_3 (Variables|Default|GetLinkedCashier))
  (bind _linkedcashier_4 (Variables|Default|GetLinkedCashier))
  (bind _linkedcashier_5 (Variables|Default|GetLinkedCashier))
  (bind _linkedcashier_6 (Variables|Default|GetLinkedCashier))
  (bind _linkedcashier_7 (Variables|Default|GetLinkedCashier))
  (bind _linkedcashier_8 (Variables|Default|GetLinkedCashier))
  (bind _linkedcashier_9 (Variables|Default|GetLinkedCashier))
  (if (Variables|Default|GetMenuButtonClicked)
    (Variables|Default|SetMenuButtonClicked false)
    (Utilities|FlowControl|Delay 1.0)
    (bind _returnvalue (Game|SpawnActorfromClass "/Game/Catcafe/meshes/BP_Beverage.BP_Beverage_C" (Math|Transform|MakeTransform (+ (Transformation|GetActorLocation) (Math|Vector|MakeVector 0.0 0.0 1e+01)) "0, 0, 0" "1.000000,1.000000,1.000000") "Undefined" "MultiplyWithRoot" 0 0))
    (Variables|/Game/Catcafe/meshes/BP_Beverage.BP_Beverage_C|SetSugar _returnvalue (Variables|/Game/Catcafe/meshes/BP_CoffeeMenu.BP_CoffeeMenu_C|Getsugar (stale OnComponentBeginOverlap(Machine) _returnvalue_2)))
    (Variables|/Game/Catcafe/meshes/BP_Beverage.BP_Beverage_C|SetCream _returnvalue (Variables|/Game/Catcafe/meshes/BP_CoffeeMenu.BP_CoffeeMenu_C|Getcream (stale OnComponentBeginOverlap(Machine) _returnvalue_2)))
    (Variables|/Game/Catcafe/meshes/BP_Beverage.BP_Beverage_C|SetType _returnvalue (Variables|/Game/Catcafe/meshes/BP_CoffeeMenu.BP_CoffeeMenu_C|Gettype (stale OnComponentBeginOverlap(Machine) _returnvalue_2)))
    (Utilities|FlowControl|Delay (Math|Conversions|ToFloat(Integer) (Variables|Default|GetCoffeeWaitTime)))
    (Transformation|SetActorLocation _returnvalue "600.000000,300.000000,90.000000" true true)
    (if (!= (Variables|/Game/Catcafe/meshes/BP_Beverage.BP_Beverage_C|GetSugar _returnvalue) 0)
      (if (!= (Variables|/Game/Catcafe/meshes/BP_Beverage.BP_Beverage_C|GetCream _returnvalue) 0)
        (if (Utilities|Enum|Equal(Enum) (Variables|/Game/Catcafe/meshes/BP_Beverage.BP_Beverage_C|GetType _returnvalue) "Coffee")
          (if (Utilities|Enum|Equal(Enum) (Variables|/Game/BP_Cashier.BP_Cashier_C|GetNPCOrder _linkedcashier_7) "Coffee. Yes Sugar. Yes Cream.")
            (Variables|/Game/BP_Cashier.BP_Cashier_C|SetOrderDelivered _linkedcashier_2 true)
            (Variables|/Game/BP_Cashier.BP_Cashier_C|SetOrderCorrect _linkedcashier_2 true)
            (Utilities|FlowControl|Delay 3.0)
            (Actor|DestroyActor _returnvalue)
            (else
              (Variables|/Game/BP_Cashier.BP_Cashier_C|SetOrderDelivered _linkedcashier_2 true)
              (Variables|/Game/BP_Cashier.BP_Cashier_C|SetOrderCorrect _linkedcashier_2 false)
              (Utilities|FlowControl|Delay 3.0)
              (Actor|DestroyActor _returnvalue)))
          (elif (Utilities|Enum|Equal(Enum) (Variables|/Game/Catcafe/meshes/BP_Beverage.BP_Beverage_C|GetType _returnvalue) "Latte")
            (if (Utilities|Enum|Equal(Enum) (Variables|/Game/BP_Cashier.BP_Cashier_C|GetNPCOrder (Variables|Default|GetLinkedCashier)) "Latte. Yes Sugar. Yes Cream.")
              (Variables|/Game/BP_Cashier.BP_Cashier_C|SetOrderDelivered _linkedcashier_9 true)
              (Variables|/Game/BP_Cashier.BP_Cashier_C|SetOrderCorrect _linkedcashier_9 true)
              (Utilities|FlowControl|Delay 3.0)
              (Actor|DestroyActor _returnvalue)
              (else
                (Variables|/Game/BP_Cashier.BP_Cashier_C|SetOrderDelivered _linkedcashier_9 true)
                (Variables|/Game/BP_Cashier.BP_Cashier_C|SetOrderCorrect _linkedcashier_9 false)
                (Utilities|FlowControl|Delay 3.0)
                (Actor|DestroyActor _returnvalue)))
            (else
              (Variables|/Game/BP_Cashier.BP_Cashier_C|SetOrderDelivered _linkedcashier_7 true)
              (Variables|/Game/BP_Cashier.BP_Cashier_C|SetOrderCorrect _linkedcashier_7 false)
              (Utilities|FlowControl|Delay 3.0)
              (Actor|DestroyActor _returnvalue)))))
      (elif (!= (Variables|/Game/Catcafe/meshes/BP_Beverage.BP_Beverage_C|GetCream _returnvalue) 0)
        (if (Utilities|Enum|Equal(Enum) (Variables|/Game/Catcafe/meshes/BP_Beverage.BP_Beverage_C|GetType _returnvalue) "Tea")
          (if (Utilities|Enum|Equal(Enum) (Variables|/Game/BP_Cashier.BP_Cashier_C|GetNPCOrder (Variables|Default|GetLinkedCashier)) "Tea. No Sugar. Yes Cream")
            (Variables|/Game/BP_Cashier.BP_Cashier_C|SetOrderDelivered _linkedcashier_3 true)
            (Variables|/Game/BP_Cashier.BP_Cashier_C|SetOrderCorrect _linkedcashier_3 true)
            (Utilities|FlowControl|Delay 3.0)
            (Actor|DestroyActor _returnvalue)
            (else
              (Variables|/Game/BP_Cashier.BP_Cashier_C|SetOrderDelivered _linkedcashier_4 true)
              (Variables|/Game/BP_Cashier.BP_Cashier_C|SetOrderCorrect _linkedcashier_4 false)
              (Utilities|FlowControl|Delay 3.0)
              (Actor|DestroyActor _returnvalue)))
          (else
            (Variables|/Game/BP_Cashier.BP_Cashier_C|SetOrderDelivered _linkedcashier_4 true)
            (Variables|/Game/BP_Cashier.BP_Cashier_C|SetOrderCorrect _linkedcashier_4 false)
            (Utilities|FlowControl|Delay 3.0)
            (Actor|DestroyActor _returnvalue)))
        (elif (Utilities|Enum|Equal(Enum) (Variables|/Game/Catcafe/meshes/BP_Beverage.BP_Beverage_C|GetType _returnvalue) "Coffee")
          (if (Utilities|Enum|Equal(Enum) (Variables|/Game/BP_Cashier.BP_Cashier_C|GetNPCOrder (Variables|Default|GetLinkedCashier)) "Coffee. No Sugar. No Cream")
            (Variables|/Game/BP_Cashier.BP_Cashier_C|SetOrderDelivered _linkedcashier_5 true)
            (Variables|/Game/BP_Cashier.BP_Cashier_C|SetOrderCorrect _linkedcashier_5 true)
            (Utilities|FlowControl|Delay 3.0)
            (Actor|DestroyActor _returnvalue)
            (else
              (Variables|/Game/BP_Cashier.BP_Cashier_C|SetOrderDelivered _linkedcashier true)
              (Variables|/Game/BP_Cashier.BP_Cashier_C|SetOrderCorrect _linkedcashier false)
              (Utilities|FlowControl|Delay 3.0)
              (Actor|DestroyActor _returnvalue)))
          (elif (Utilities|Enum|Equal(Enum) (Variables|/Game/Catcafe/meshes/BP_Beverage.BP_Beverage_C|GetType _returnvalue) "Latte")
            (if (Utilities|Enum|Equal(Enum) (Variables|/Game/BP_Cashier.BP_Cashier_C|GetNPCOrder (Variables|Default|GetLinkedCashier)) "Latte. No Sugar. No Cream")
              (Variables|/Game/BP_Cashier.BP_Cashier_C|SetOrderDelivered _linkedcashier_6 true)
              (Variables|/Game/BP_Cashier.BP_Cashier_C|SetOrderCorrect _linkedcashier_6 true)
              (Utilities|FlowControl|Delay 3.0)
              (Actor|DestroyActor _returnvalue)
              (else
                (Variables|/Game/BP_Cashier.BP_Cashier_C|SetOrderDelivered _linkedcashier_6 true)
                (Variables|/Game/BP_Cashier.BP_Cashier_C|SetOrderCorrect _linkedcashier_6 false)
                (Utilities|FlowControl|Delay 3.0)
                (Actor|DestroyActor _returnvalue)))
            (elif (Utilities|Enum|Equal(Enum) (Variables|/Game/Catcafe/meshes/BP_Beverage.BP_Beverage_C|GetType _returnvalue) "Tea")
              (if (Utilities|Enum|Equal(Enum) (Variables|/Game/BP_Cashier.BP_Cashier_C|GetNPCOrder (Variables|Default|GetLinkedCashier)) "Tea. No Sugar. No Cream")
                (Variables|/Game/BP_Cashier.BP_Cashier_C|SetOrderDelivered _linkedcashier_8 true)
                (Variables|/Game/BP_Cashier.BP_Cashier_C|SetOrderCorrect _linkedcashier_8 true)
                (Utilities|FlowControl|Delay 3.0)
                (Actor|DestroyActor _returnvalue)
                (else
                  (Variables|/Game/BP_Cashier.BP_Cashier_C|SetOrderDelivered _linkedcashier_8 true)
                  (Variables|/Game/BP_Cashier.BP_Cashier_C|SetOrderCorrect _linkedcashier_8 false)
                  (Utilities|FlowControl|Delay 3.0)
                  (Actor|DestroyActor _returnvalue)))
              (else
                (Variables|/Game/BP_Cashier.BP_Cashier_C|SetOrderDelivered _linkedcashier_8 true)
                (Variables|/Game/BP_Cashier.BP_Cashier_C|SetOrderCorrect _linkedcashier_8 false)
                (Utilities|FlowControl|Delay 3.0)
                (Actor|DestroyActor _returnvalue)))))))))

(fn ConstructionScript)