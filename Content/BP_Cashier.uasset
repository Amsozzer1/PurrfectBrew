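; Cashier Blueprint that registers itself as the LinkedCashier on coffee machines and NPCs.
; On BeginPlay it finds every BP_CoffeeMachine and sets that reference.
; Every Tick it repeats a world-wide search for NPC_Blueprint actors and reassigns itself to each.
; Tick also branches on OrderDelivered and OrderCorrect, but neither outcome triggers any logic yet.
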(event EventBeginPlay
  (bind _outactors (Actor|GetAllActorsOfClass "/Game/Catcafe/meshes/BP_CoffeeMachine.BP_CoffeeMachine_C"))
  (for _array_element _outactors
    (Variables|/Game/Catcafe/meshes/BP_CoffeeMachine.BP_CoffeeMachine_C|SetLinkedCashier _array_element self)))

(event Collision|EventActorBeginOverlap
  (params (OtherActor :type Actor%20Object%20Reference)))

(event EventTick
  (params (DeltaSeconds :type Float%20%28single-precision%29))
  (Utilities|FlowControl|Sequence
    (:then_0
      (bind _outactors (Actor|GetAllActorsOfClass "/Game/Actor_Blueprints/NPC_Blueprint.NPC_Blueprint_C"))
      (for _array_element _outactors
        (Variables|/Game/Actor_Blueprints/NPC_Blueprint.NPC_Blueprint_C|SetLinkedCashier _array_element self)))
    (:then_1
      (if (Variables|Default|GetOrderDelivered)
        (if (Variables|Default|GetOrderCorrect)
          _)))))

(fn ConstructionScript)